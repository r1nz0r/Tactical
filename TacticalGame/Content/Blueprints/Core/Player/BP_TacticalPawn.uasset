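; Player camera pawn for a tactical game, providing pan, stepped rotation and spring-arm zoom through Enhanced Input.
; On BeginPlay it adds the tactical mapping context and seeds desired zoom, location and rotation from current values.
; Input only changes these targets: clamped zoom, 45-degree yaw steps, and moves relative to actor facing.
; Tick interpolates spring arm length and actor transform toward the targets for smooth motion, without collision sweep.
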(event Input|EnhancedActionEvents|EnhancedInputActionIA_ZoomCamera
  (params (ActionValue :type Float%20%28double-precision%29) (ElapsedSeconds :type Float%20%28double-precision%29) (TriggeredSeconds :type Float%20%28double-precision%29) (InputAction :type Input%20Action%20Object%20Reference :default "/Game/Blueprints/IA_ZoomCamera.IA_ZoomCamera"))
  (:Triggered
    (CallFunction|SetDesiredZoom ActionValue)))

(event Input|EnhancedActionEvents|EnhancedInputActionIA_Move
  (params (ActionValue :type Vector%202D%20Structure) (ElapsedSeconds :type Float%20%28double-precision%29) (TriggeredSeconds :type Float%20%28double-precision%29) (InputAction :type Input%20Action%20Object%20Reference :default "/Game/Blueprints/IA_Move.IA_Move"))
  (:Triggered
    (CallFunction|SetDesiredLocation (.x ActionValue) (.y ActionValue))))

(event Input|EnhancedActionEvents|EnhancedInputActionIA_RotateCamera
  (params (ActionValue :type Float%20%28double-precision%29) (ElapsedSeconds :type Float%20%28double-precision%29) (TriggeredSeconds :type Float%20%28double-precision%29) (InputAction :type Input%20Action%20Object%20Reference :default "/Game/Blueprints/IA_RotateCamera.IA_RotateCamera"))
  (:Started
    (CallFunction|SetDesiredRotation ActionValue)))

(event EventBeginPlay
  (CallFunction|AddEnhancedInputSystem)
  (CallFunction|InitializeDesiredZoom)
  (CallFunction|InitializeDesiredLocation)
  (CallFunction|InitializeDesiredRotation))

(event EventTick
  (params (DeltaSeconds :type Float%20%28single-precision%29))
  (CallFunction|UpdateZoom (Variables|Zoom|GetZoomInterpSpeed))
  (CallFunction|UpdateLocation (Variables|Movement|GetMoveInterpSpeed))
  (CallFunction|UpdateRotation (Variables|Default|GetRotationInterpSpeed)))

(fn ConstructionScript)

(fn AddEnhancedInputSystem
  (bind _asbp_tactical_player_controller (Utilities|Casting|CastToBP_TacticalPlayerController (Game|GetPlayerController 0)))
  (Input|AddMappingContext (PlayerController|LocalPlayerSubsystems|GetEnhancedInputLocalPlayerSubsystem _asbp_tactical_player_controller) "/Game/Blueprints/IM_Tactical.IM_Tactical" 0 "(bIgnoreAllPressedKeysUntilRelease=True,bForceImmediately=False)"))

(fn SetDesiredZoom
  (params (A :type Float%20%28double-precision%29))
  (bind _zoomclamp (Variables|Zoom|GetZoomClamp))
  (Variables|Zoom|SetDesiredZoom (Math|Float|Clamp(Float) (+ (* A 4e+01) (Variables|Zoom|GetDesiredZoom)) (.x _zoomclamp) (.y _zoomclamp))))

(fn InitializeDesiredZoom
  (Variables|Zoom|SetDesiredZoom (Variables|/Script/Engine.SpringArmComponent|GetTargetArmLength (Variables|Default|GetSpringArm))))

(fn UpdateZoom
  (params (InterSpeed :type Float%20%28double-precision%29))
  (Variables|/Script/Engine.SpringArmComponent|SetTargetArmLength (Variables|Default|GetSpringArm) (Math|Interpolation|FInterpTo (Variables|/Script/Engine.SpringArmComponent|GetTargetArmLength (Variables|Default|GetSpringArm)) (Variables|Zoom|GetDesiredZoom) (Utilities|Time|GetWorldDeltaSeconds) InterSpeed)))

(fn UpdateLocation
  (params (MovementInterpSpeed :type Float%20%28double-precision%29))
  (Transformation|SetActorLocation (Math|Interpolation|VInterpTo (Transformation|GetActorLocation) (Variables|Movement|GetDesiredLocation) (Utilities|Time|GetWorldDeltaSeconds) MovementInterpSpeed) false false))

(fn InitializeDesiredLocation
  (Variables|Movement|SetDesiredLocation (Transformation|GetActorLocation)))

(fn UpdateRotation
  (params (RotationInterpSpeed :type Float%20%28double-precision%29))
  (Transformation|SetActorRotation (Math|Interpolation|RInterpTo (Transformation|GetActorRotation) (Variables|Default|GetDesiredRotation) (Utilities|Time|GetWorldDeltaSeconds) RotationInterpSpeed)))

(fn SetDesiredRotation
  (params (A :type Float%20%28double-precision%29))
  (Variables|Default|SetDesiredRotation (Math|Rotator|CombineRotators (Variables|Default|GetDesiredRotation) (Math|Rotator|MakeRotator 0.0 0.0 (* A 45.0)))))

(fn InitializeDesiredRotation
  (Variables|Default|SetDesiredRotation (Transformation|GetActorRotation)))

(fn SetDesiredLocation
  (params (X :type Float%20%28double-precision%29) (Y :type Float%20%28double-precision%29))
  (Variables|Movement|SetDesiredLocation (+ (Variables|Movement|GetDesiredLocation) (* (+ (* X (Transformation|GetActorForwardVector)) (* Y (Transformation|GetActorRightVector))) (Variables|Movement|GetMoveStep)))))